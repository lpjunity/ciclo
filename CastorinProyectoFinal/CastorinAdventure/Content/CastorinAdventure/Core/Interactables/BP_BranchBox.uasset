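; BP_BranchBox is an interactable box where the player deposits carried branches.
; On Interact, a BP_Branch item is attached to the box mesh at the socket matching its ItemName, so each branch's name selects its slot.
; It then plays a deposit sound, notifies the interacting actor through CallOnBranchPlaced and clears that actor's Pickeable reference.
; Any other item only prints a wrong-item message.
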(event `/Game/CastorinAdventure/Core/Interactables/BPI_Interactable.Interact`
  (params (InteractItem :type "Actor Object Reference") (InteractActor :type "/Game/CastorinAdventure/Core/Characters/BP_Castorin Object Reference") (interactStructure :type "Actor Object Reference"))
  (`parent.Interact` InteractItem InteractActor interactStructure)
  (bind _asbp_branch (cast `/Game/CastorinAdventure/Core/Pickups/BP_Branch` InteractItem)
    (:`then`
      (`self.AttachInPlace` _asbp_branch (`self.StaticMesh`) (`/Game/CastorinAdventure/Core/Pickups/BP_PhysicsObject.ItemName` _asbp_branch))
      (`GameplayStatics.PlaySound2D` "/Game/CastorinAdventure/Sounds/FX/Beefy_Hit_With_Object_DepositarPaloEnCajaB.Beefy_Hit_With_Object_DepositarPaloEnCajaB" 0.5 1.0 0.0 null null)
      (`/Game/CastorinAdventure/Core/Characters/BP_Castorin.OnBranchPlaced` InteractActor _asbp_branch)
      (set `/Game/CastorinAdventure/Core/Characters/BP_Castorin.Pickeable` null InteractActor))
    (:`CastFailed`
      (`KismetSystemLibrary.PrintString` (`self.WrongItemMessage`)))))

(fn `UserConstructionScript`
  (`parent.UserConstructionScript`))