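; BP_Bookshelf is an interactable bookshelf where the player places books they are carrying.
; On Interact, it casts the item to BP_Book and attaches it to the shelf mesh at the socket named after the book's ItemName.
; It then plays a placement sound, notifies the interacting actor via CallOnBookPlaced, and clears that actor's Pickeable reference.
; Any other item just prints a wrong-item message.
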(event `/Game/CastorinAdventure/Core/Interactables/BPI_Interactable.Interact`
  (params (InteractItem :type "Actor Object Reference") (InteractActor :type "/Game/CastorinAdventure/Core/Characters/BP_Castorin Object Reference") (interactStructure :type "Actor Object Reference"))
  (`parent.Interact` InteractItem InteractActor interactStructure)
  (bind _asbp_book (cast `/Game/CastorinAdventure/Core/Pickups/BP_Book` InteractItem)
    (:`then`
      (`self.AttachInPlace` _asbp_book (`self.StaticMesh`) (`/Game/CastorinAdventure/Core/Pickups/BP_PhysicsObject.ItemName` _asbp_book))
      (`GameplayStatics.PlaySound2D` "/Game/CastorinAdventure/Sounds/FX/Hit_Jacket_Light_C_DepositarLibroA.Hit_Jacket_Light_C_DepositarLibroA" 0.5 1.0 0.0 null null)
      (`/Game/CastorinAdventure/Core/Characters/BP_Castorin.OnBookPlaced` InteractActor _asbp_book)
      (set `/Game/CastorinAdventure/Core/Characters/BP_Castorin.Pickeable` null InteractActor))
    (:`CastFailed`
      (`KismetSystemLibrary.PrintString` (`self.WrongItemMessage`)))))

(fn `UserConstructionScript`
  (`parent.UserConstructionScript`))