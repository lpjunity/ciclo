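; BP_PhysicsObject is a physics pickup that can be grabbed and dropped by a character.
; Grab disables physics simulation and collision on the mesh and sphere, then snaps the object to a named socket on the character's mesh.
; Drop restores collision, re-enables physics and detaches the mesh in place, with the sphere query-only.
; Both events print debug strings for attach and detach.
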(event `/Game/CastorinAdventure/Core/Pickups/BPI_Grabeable.Grab`
  (params (Character :type "/Game/CastorinAdventure/Core/Characters/BP_Castorin Object Reference (by ref)"))
  (bind _mesh (`self.Mesh`))
  (`PrimitiveComponent.SetSimulatePhysics` _mesh false)
  (`PrimitiveComponent.SetCollisionEnabled` _mesh "NoCollision")
  (`PrimitiveComponent.SetCollisionEnabled` (`self.Sphere`) "NoCollision")
  (bind _returnvalue (`self.K2_AttachToComponent` (`Character.Mesh` Character) (`self.SocketName`) "SnapToTarget" "SnapToTarget" "KeepWorld" false))
  (if _returnvalue
    (`KismetSystemLibrary.PrintString` "Attached!" true true (struct :`G` 0.66 :`B` 1.0 :`A` 1.0) 2.0 "4")
    (else
      (`KismetSystemLibrary.PrintString` "Not Attached!" true true (struct :`G` 0.66 :`B` 1.0 :`A` 1.0) 2.0 "7"))))

(event `/Game/CastorinAdventure/Core/Pickups/BPI_Grabeable.Drop`
  (bind _mesh (`self.Mesh`))
  (`PrimitiveComponent.SetCollisionEnabled` _mesh "QueryAndPhysics")
  (`PrimitiveComponent.SetCollisionEnabled` (`self.Sphere`) "QueryOnly")
  (`PrimitiveComponent.SetSimulatePhysics` _mesh true)
  (`SceneComponent.K2_DetachFromComponent` (`self.Mesh`) "KeepWorld" "KeepWorld" "KeepWorld" true)
  (`KismetSystemLibrary.PrintString` "Dettached!" true true (struct :`G` 0.66 :`B` 1.0 :`A` 1.0) 2.0 "6"))

(fn `UserConstructionScript`)